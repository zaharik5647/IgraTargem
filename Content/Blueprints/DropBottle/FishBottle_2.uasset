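; FishBottle_2 is a hazard Blueprint that damages the 2D side-scroller character on contact and then removes itself.
; Its Sphere1 overlap reacts only to that character's capsule component, briefly pulsing the character's Hit flag.
; After the short delay it subtracts a fixed amount from the character's Health and destroys the bottle actor.
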(event OnComponentBeginOverlap(Sphere1)
  (params (OverlappedComponent :type Primitive%20Component%20Object%20Reference) (OtherActor :type Actor%20Object%20Reference) (OtherComp :type Primitive%20Component%20Object%20Reference) (OtherBodyIndex :type Integer) (bFromSweep :type Boolean) (SweepResult :type Hit%20Result%20Structure%20%28by%20ref%29))
  (Utilities|FlowControl|Sequence
    (:then_0
      (bind _as2dside_scroller_character (Utilities|Casting|CastTo2DSideScrollerCharacter OtherActor))
      (if (== OtherComp (Variables|/Script/Engine.Character|GetCapsuleComponent _as2dside_scroller_character))
        (Variables|/Game/Blueprints/2DSideScrollerCharacter.2DSideScrollerCharacter_C|SetHit _as2dside_scroller_character true)
        (Utilities|FlowControl|Delay 0.05)
        (Variables|/Game/Blueprints/2DSideScrollerCharacter.2DSideScrollerCharacter_C|SetHit _as2dside_scroller_character false)
        (Variables|/Game/Blueprints/2DSideScrollerCharacter.2DSideScrollerCharacter_C|SetHealth _as2dside_scroller_character (- (Variables|/Game/Blueprints/2DSideScrollerCharacter.2DSideScrollerCharacter_C|GetHealth _as2dside_scroller_character) 3))
        (Actor|DestroyActor)))))

(event EventBeginPlay)

(event Collision|EventActorBeginOverlap
  (params (OtherActor :type Actor%20Object%20Reference)))

(event EventTick
  (params (DeltaSeconds :type Float%20%28single-precision%29)))

(fn ConstructionScript)