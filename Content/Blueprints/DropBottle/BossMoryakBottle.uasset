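; BossMoryakBottle is a damaging bottle hazard, apparently tied to the sailor boss.
; When Sphere1 overlaps the capsule of either player class, 2DSideScrollerCharacter or Igrok4Uroven, it plays a damage sound and briefly pulses that player's Hit flag.
; It then subtracts one Health and destroys itself.
; Both classes use duplicated cast branches, and the file contains no movement logic.
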(event OnComponentBeginOverlap(Sphere1)
  (params (OverlappedComponent :type Primitive%20Component%20Object%20Reference) (OtherActor :type Actor%20Object%20Reference) (OtherComp :type Primitive%20Component%20Object%20Reference) (OtherBodyIndex :type Integer) (bFromSweep :type Boolean) (SweepResult :type Hit%20Result%20Structure%20%28by%20ref%29))
  (Utilities|FlowControl|Sequence
    (:then_0
      (bind _as2dside_scroller_character (Utilities|Casting|CastTo2DSideScrollerCharacter OtherActor))
      (if (== OtherComp (Variables|/Script/Engine.Character|GetCapsuleComponent _as2dside_scroller_character))
        (Audio|SpawnSound2D "/Game/Sounds/Герой/Получение_урона_Cue.Получение_урона_Cue" 1.0 1.0 0.0 0)
        (Variables|/Game/Blueprints/2DSideScrollerCharacter.2DSideScrollerCharacter_C|SetHit _as2dside_scroller_character true)
        (Utilities|FlowControl|Delay 0.05)
        (Variables|/Game/Blueprints/2DSideScrollerCharacter.2DSideScrollerCharacter_C|SetHit _as2dside_scroller_character false)
        (Variables|/Game/Blueprints/2DSideScrollerCharacter.2DSideScrollerCharacter_C|SetHealth _as2dside_scroller_character (- (Variables|/Game/Blueprints/2DSideScrollerCharacter.2DSideScrollerCharacter_C|GetHealth _as2dside_scroller_character) 1))
        (Actor|DestroyActor)))
    (:then_1
      (bind _asigrok_4uroven (Utilities|Casting|CastToIgrok4Uroven OtherActor))
      (if (== (Variables|/Script/Engine.Character|GetCapsuleComponent _asigrok_4uroven) OtherComp)
        (Audio|SpawnSound2D "/Game/Sounds/Герой/Получение_урона_Cue.Получение_урона_Cue" 1.0 1.0 0.0 0)
        (Variables|/Game/Blueprints/Igrok4Uroven.Igrok4Uroven_C|SetHit _asigrok_4uroven true)
        (Utilities|FlowControl|Delay 0.05)
        (Variables|/Game/Blueprints/Igrok4Uroven.Igrok4Uroven_C|SetHit _asigrok_4uroven false)
        (Variables|/Game/Blueprints/Igrok4Uroven.Igrok4Uroven_C|SetHealth _asigrok_4uroven (- (Variables|/Game/Blueprints/Igrok4Uroven.Igrok4Uroven_C|GetHealth _asigrok_4uroven) 1))
        (Actor|DestroyActor)))))

(event EventBeginPlay)

(event Collision|EventActorBeginOverlap
  (params (OtherActor :type Actor%20Object%20Reference)))

(event EventTick
  (params (DeltaSeconds :type Float%20%28single-precision%29)))

(fn ConstructionScript)