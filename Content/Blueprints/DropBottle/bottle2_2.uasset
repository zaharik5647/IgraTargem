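; Bottle projectile actor (DropBottle) that damages enemies and bosses on contact.
; When its sphere begins overlapping, a sequence of casts checks for two Ocherednyara enemy types and the Cucumber, Fish, Tomato and Moriak bosses.
; Only a hit on the target's capsule counts: it lowers Health by a per-type amount and destroys the bottle.
; Boss hits also play a 2D sound and set the boss's Hit flag.
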(event OnComponentBeginOverlap(Sphere1)
  (params (OverlappedComponent :type Primitive%20Component%20Object%20Reference) (OtherActor :type Actor%20Object%20Reference) (OtherComp :type Primitive%20Component%20Object%20Reference) (OtherBodyIndex :type Integer) (bFromSweep :type Boolean) (SweepResult :type Hit%20Result%20Structure%20%28by%20ref%29))
  (Utilities|FlowControl|Sequence
    (:then_0
      (bind _asocherednyara (Utilities|Casting|CastToOcherednyara OtherActor))
      (if (== OtherComp (Variables|/Game/Blueprints/Ocherednyara.Ocherednyara_C|GetCapsule _asocherednyara))
        (Variables|/Game/Blueprints/Ocherednyara.Ocherednyara_C|SetHealth _asocherednyara (- (Variables|/Game/Blueprints/Ocherednyara.Ocherednyara_C|GetHealth _asocherednyara) 1))
        (Actor|DestroyActor)))
    (:then_1
      (bind _asocherednyara_3 (Utilities|Casting|CastToOcherednyara_3 OtherActor))
      (if (== OtherComp (Variables|/Game/Blueprints/Ocherednyara_3.Ocherednyara_3_C|GetCapsule _asocherednyara_3))
        (Variables|/Game/Blueprints/Ocherednyara_3.Ocherednyara_3_C|SetHealth _asocherednyara_3 (- (Variables|/Game/Blueprints/Ocherednyara_3.Ocherednyara_3_C|GetHealth _asocherednyara_3) 1))
        (Actor|DestroyActor)))
    (:then_2
      (bind _ascucumber_boss (Utilities|Casting|CastToCucumberBoss OtherActor))
      (if (== OtherComp (Variables|/Game/Blueprints/CucumberBoss.CucumberBoss_C|GetCapsule _ascucumber_boss))
        (Audio|SpawnSound2D "/Game/Sounds/враги/первая_-_5_Cue.первая_-_5_Cue" 1.0 1.0 0.0 0)
        (Variables|/Game/Blueprints/CucumberBoss.CucumberBoss_C|SetHealth _ascucumber_boss (- (Variables|/Game/Blueprints/CucumberBoss.CucumberBoss_C|GetHealth _ascucumber_boss) 3))
        (Variables|/Game/Blueprints/CucumberBoss.CucumberBoss_C|Sethit _ascucumber_boss true)
        (Actor|DestroyActor)))
    (:then_3
      (bind _asfish_boss (Utilities|Casting|CastToFishBoss OtherActor))
      (if (== (Variables|/Game/Blueprints/FishBoss.FishBoss_C|GetCapsule _asfish_boss) OtherComp)
        (Audio|SpawnSound2D "/Game/Sounds/враги/первая_-_3_Cue.первая_-_3_Cue" 1.0 1.0 0.0 0)
        (Variables|/Game/Blueprints/FishBoss.FishBoss_C|SetHealth _asfish_boss (- (Variables|/Game/Blueprints/FishBoss.FishBoss_C|GetHealth _asfish_boss) 3))
        (Variables|/Game/Blueprints/FishBoss.FishBoss_C|Sethit _asfish_boss true)
        (Actor|DestroyActor)))
    (:then_4
      (bind _astomato_boss (Utilities|Casting|CastToTomatoBoss OtherActor))
      (if (== (Variables|/Game/Blueprints/TomatoBoss.TomatoBoss_C|GetCapsule _astomato_boss) OtherComp)
        (Audio|SpawnSound2D "/Game/Sounds/враги/первая_-_3_Cue.первая_-_3_Cue" 1.0 1.0 0.0 0)
        (Variables|/Game/Blueprints/TomatoBoss.TomatoBoss_C|SetHealth _astomato_boss (- (Variables|/Game/Blueprints/TomatoBoss.TomatoBoss_C|GetHealth _astomato_boss) 3))
        (Variables|/Game/Blueprints/TomatoBoss.TomatoBoss_C|Sethit _astomato_boss true)
        (Actor|DestroyActor)))
    (:then_5
      (bind _asmoriak_boss (Utilities|Casting|CastToMoriakBoss OtherActor))
      (if (== (Variables|/Game/Blueprints/MoriakBoss.MoriakBoss_C|GetCapsule _asmoriak_boss) OtherComp)
        (Audio|SpawnSound2D "/Game/Sounds/враги/первая_-_3_Cue.первая_-_3_Cue" 1.0 1.0 0.0 0)
        (Variables|/Game/Blueprints/MoriakBoss.MoriakBoss_C|SetHealth _asmoriak_boss (- (Variables|/Game/Blueprints/MoriakBoss.MoriakBoss_C|GetHealth _asmoriak_boss) 1))
        (Variables|/Game/Blueprints/MoriakBoss.MoriakBoss_C|Sethit _asmoriak_boss true)
        (Actor|DestroyActor)))))

(event EventBeginPlay)

(event Collision|EventActorBeginOverlap
  (params (OtherActor :type Actor%20Object%20Reference)))

(event EventTick
  (params (DeltaSeconds :type Float%20%28single-precision%29)))

(fn ConstructionScript)