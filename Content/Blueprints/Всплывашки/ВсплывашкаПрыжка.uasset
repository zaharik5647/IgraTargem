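; One-shot trigger actor that shows the jump popup widget (ВсплывашкаПрыжка) when the 2DSideScrollerCharacter enters its Box.
; The overlap creates the widget if needed, adds it to the viewport, pauses the game, shows the cursor and switches to Game and UI input.
; If the game is already paused, it instead removes the widget, unpauses and restores game-only input.
; Either branch ends by destroying the actor.
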(event OnComponentBeginOverlap(Box)
  (params (OverlappedComponent :type Primitive%20Component%20Object%20Reference) (OtherActor :type Actor%20Object%20Reference) (OtherComp :type Primitive%20Component%20Object%20Reference) (OtherBodyIndex :type Integer) (bFromSweep :type Boolean) (SweepResult :type Hit%20Result%20Structure%20%28by%20ref%29))
  (bind _returnvalue (Game|GetPlayerController 0))
  (Utilities|Casting|CastTo2DSideScrollerCharacter OtherActor)
  (Utilities|IsValid (Variables|Default|GetNewVar_0)
    (:Is%20Valid
      _)
    (:Is%20Not%20Valid
      (bind _returnvalue_2 (UserInterface|CreateWidget "/Game/UI/Всплывашки/ВсплывашкаПрыжка.ВсплывашкаПрыжка_C"))
      (Variables|Default|SetNewVar_0 _returnvalue_2)))
  (if (Game|IsGamePaused)
    (Widget|RemovefromParent (Variables|Default|GetNewVar_0))
    (Game|SetGamePaused false)
    (Variables|/Script/Engine.PlayerController|SetbShowMouseCursor _returnvalue false)
    (Input|SetInputModeGameOnly _returnvalue)
    (else
      (UserInterface|Viewport|AddtoViewport (Variables|Default|GetNewVar_0) 0)
      (Game|SetGamePaused true)
      (Variables|/Script/Engine.PlayerController|SetbShowMouseCursor _returnvalue true)
      (Input|SetInputModeGameandUI _returnvalue (Variables|Default|GetNewVar_0) "LockInFullscreen" false)))
  (Actor|DestroyActor))

(event EventBeginPlay)

(event Collision|EventActorBeginOverlap
  (params (OtherActor :type Actor%20Object%20Reference)))

(event EventTick
  (params (DeltaSeconds :type Float%20%28single-precision%29)))

(fn ConstructionScript)