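; Level-exit trigger actor that moves the 2D side-scroller character on to ThirdLevel.
; On box overlap, it loads the "Save" slot, sets Level2Complete, calls save with no object connected, then opens the level, unpauses and restores game-only input with a hidden cursor.
; If no save exists, it only writes a fresh save object, without marking completion or changing level.
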(event OnComponentBeginOverlap(Box)
  (params (OverlappedComponent :type Primitive%20Component%20Object%20Reference) (OtherActor :type Actor%20Object%20Reference) (OtherComp :type Primitive%20Component%20Object%20Reference) (OtherBodyIndex :type Integer) (bFromSweep :type Boolean) (SweepResult :type Hit%20Result%20Structure%20%28by%20ref%29))
  (bind _returnvalue (Game|GetPlayerController 0))
  (Utilities|Casting|CastTo2DSideScrollerCharacter OtherActor)
  (bind _returnvalue_2 (SaveGame|CreateSaveGameObject "/Game/SaveGame/Save.Save_C"))
  (bind _output_get (Variables|Default|SetNewVar_2 _returnvalue_2))
  (bind _returnvalue_3 (SaveGame|DoesSaveGameExist "Save"))
  (if _returnvalue_3
    (bind _returnvalue_4 (SaveGame|LoadGamefromSlot "Save"))
    (bind _assave (Utilities|Casting|CastToSave _returnvalue_4))
    (bind _output_get_2 (Variables|Default|SetAs%20Save _assave))
    (Variables|/Game/SaveGame/Save.Save_C|SetLevel2Complete _output_get_2 true)
    (SaveGame|SaveGametoSlot 0 "Save")
    (Game|OpenLevel(byName) "ThirdLevel")
    (Game|SetGamePaused false)
    (Input|SetInputModeGameOnly _returnvalue)
    (Variables|/Script/Engine.PlayerController|SetbShowMouseCursor _returnvalue false)
    (else
      (SaveGame|SaveGametoSlot _output_get "Save"))))

(event EventBeginPlay)

(event Collision|EventActorBeginOverlap
  (params (OtherActor :type Actor%20Object%20Reference)))

(event EventTick
  (params (DeltaSeconds :type Float%20%28single-precision%29)))

(fn ConstructionScript)